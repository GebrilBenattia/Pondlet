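; BP_WaterLily is a water lily add-on that spawns a frog shortly after play begins.
; BeginPlay calls its parent, then sets a one-shot timer by function name for SpawnAnimal.
; SpawnAnimal runs the parent version, triggers spawn VFX, then spawns an enlarged BP_FrogTMP at the lily's location with random rotation and records it in SpawnedActors.
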(event `self.ReceiveBeginPlay`
  (`parent.ReceiveBeginPlay`)
  (`KismetSystemLibrary.K2_SetTimer` null "SpawnAnimal" 5.0))

(fn `SpawnAnimal`
  (bind _returnvalue_location (`KismetMathLibrary.BreakTransform` (`self.GetTransform`)))
  (`parent.SpawnAnimal`)
  (`self.CallSpawnVFX`)
  (bind _returnvalue (`|SpawnActorFromClass` "/Game/Blueprints/AI/Species/BP_FrogTMP.BP_FrogTMP_C" (`KismetMathLibrary.MakeTransform` _returnvalue_location (`self.RandRot`) (3.5 3.5 3.5)) "Undefined" "MultiplyWithRoot" null null))
  (`KismetArrayLibrary.Array_Add` (`self.SpawnedActors`) _returnvalue))

(fn `UserConstructionScript`
  (`parent.UserConstructionScript`))
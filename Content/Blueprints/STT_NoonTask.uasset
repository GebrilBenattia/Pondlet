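; StateTree task for the Noon state of the day cycle, rotating the sun and moon directional lights as time passes.
; On enter it caches BP_DayCycleSystem; each tick it finds lights by Sun/Moon tags and looks up the Noon settings.
; The 24-hour time becomes an alpha, wrapping past midnight, that lerps sun roll between start and end angles.
; The moon sits 180 degrees opposite, and out-of-range hours leave both untouched.
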(event `self.ReceiveLatentEnterState`
  (params (Transition :type "StateTreeTransitionResult Structure (by ref)"))
  (`KismetSystemLibrary.PrintString` "Noon task Start")
  (bind _returnvalue (`GameplayStatics.GetActorOfClass` "/Game/Blueprints/BP_DayCycleSystem.BP_DayCycleSystem_C"))
  (set `self.DayCYcle` _returnvalue))

(event `self.ReceiveLatentTick`
  (params (DeltaTime :type "Float (single-precision)"))
  (`self.RotateLight`))

(event `self.ReceiveExitState`
  (params (Transition :type "StateTreeTransitionResult Structure (by ref)"))
  (`KismetSystemLibrary.PrintString` "ExitNoon"))

(fn `GetDayStateSettingFromName`
  (params (DayStates :type "Array of DayStateSettings Structure") (Name :type Name))
  (returns (DayState :type "DayStateSettings Structure") (IsFound :type Boolean))
  (locals (IsFoundVar :type Boolean) (State :type "DayStateSettings Structure") (NameVar :type Name))
  (set `local.NameVar` Name)
  (for _array_element DayStates
    (if (== (`.DayStateName` (break `DayStateSettings` _array_element)) (`local.NameVar`))
      (set `local.State` _array_element)
      (set `local.IsFoundVar` true)
      (break)))
  (return (`local.State`) (`local.IsFoundVar`)))

(fn `GetLerpValueBetweenHours`
  (params (Start :type "Float (double-precision)") (End :type "Float (double-precision)") (CurrentHour :type "Float (double-precision)"))
  (returns (ReturnValue :type "Float (double-precision)"))
  (locals (StartV :type "Float (double-precision)") (EndV :type "Float (double-precision)") (CurrentHourV :type "Float (double-precision)"))
  (bind _returnvalue (`KismetMathLibrary.MapRangeUnclamped` (`local.CurrentHourV`) (`local.StartV`) (`local.EndV`) 0.0 1.0))
  (set `local.StartV` Start)
  (set `local.EndV` End)
  (set `local.CurrentHourV` CurrentHour)
  (`|ExecutionSequence`
    (:`then_0`
      (if (> (`local.StartV`) (`local.EndV`))
        (set `local.EndV` (+ (`local.EndV`) 24.0))))
    (:`then_1`
      (if (> (`local.StartV`) (`local.CurrentHourV`))
        (set `local.CurrentHourV` (+ (`local.CurrentHourV`) 24.0))))
    (:`then_2`
      (if (`KismetMathLibrary.InRange_FloatFloat` (`local.CurrentHourV`) (`local.StartV`) (`local.EndV`))
        (`KismetSystemLibrary.PrintString` (`KismetStringLibrary.Concat_StrStr` "In : " (`KismetStringLibrary.Conv_DoubleToString` (`local.StartV`)) " " (`KismetStringLibrary.Conv_DoubleToString` (`local.EndV`)) " " (`KismetStringLibrary.Conv_DoubleToString` (`local.CurrentHourV`)) " | Out : " (`KismetStringLibrary.Conv_DoubleToString` _returnvalue)) true true (struct :`R` 0.964167 :`G` 0.952493 :`B` 1.0 :`A` 1.0) 2.0 "LerpHours")
        (return _returnvalue)
        (else
          (`KismetSystemLibrary.PrintString` (`KismetStringLibrary.Concat_StrStr` "In : " (`KismetStringLibrary.Conv_DoubleToString` (`local.StartV`)) " " (`KismetStringLibrary.Conv_DoubleToString` (`local.EndV`)) " " (`KismetStringLibrary.Conv_DoubleToString` (`local.CurrentHourV`)) " | Out : " "-1") true true (struct :`R` 0.964167 :`G` 0.952493 :`B` 1.0 :`A` 1.0) 2.0 "LerpHours")
          (return -1.0))))))

(fn `GetLights`
  (returns (SunLightRes :type "DirectionalLight Object Reference") (MoonLightRes :type "DirectionalLight Object Reference"))
  (locals (SunLight :type "DirectionalLight Object Reference") (MoonLight :type "DirectionalLight Object Reference"))
  (bind _outactors (`GameplayStatics.GetAllActorsOfClass` "/Script/Engine.DirectionalLight"))
  (for _array_element _outactors
    (bind _tags (`Actor.Tags` _array_element))
    (if (`KismetArrayLibrary.Array_Contains` _tags "Sun")
      (set `local.SunLight` _array_element)
      (elif (`KismetArrayLibrary.Array_Contains` _tags "Moon")
        (set `local.MoonLight` _array_element))))
  (return (`local.SunLight`) (`local.MoonLight`)))

(fn `RotateLight`
  (locals (MoonLight :type "DirectionalLight Object Reference") (Sunlight :type "DirectionalLight Object Reference"))
  (`|ExecutionSequence`
    (:`then_0`
      (bind (_sunlightres _moonlightres) (`self.GetLights`))
      (set `local.Sunlight` _sunlightres)
      (set `local.MoonLight` _moonlightres))
    (:`then_1`
      (bind (_daystate _isfound) (`self.GetDayStateSettingFromName` (`DayCycleSettings.DayStatesSettings` (`self.NewVar`)) "Noon"))
      (if _isfound
        (bind _sunlight (`local.Sunlight`)
          (:`then`
            (bind ((`Start24HourFormat` _start24hourformat) (`End24HourFormat` _end24hourformat) (`StartLightAngle` _startlightangle) (`EndLightAngle` _endlightangle)) (break `DayStateSettings` _daystate))
            (bind _returnvalue (`self.GetLerpValueBetweenHours` _start24hourformat _end24hourformat (`TimeManager.Time24Format` (`DayCycleSystem.TimeManager` (`self.DayCYcle`)))))
            (if (!= _returnvalue -1.0)
              (bind _returnvalue_2 (`KismetMathLibrary.Lerp` _startlightangle _endlightangle _returnvalue))
              (`Actor.K2_SetActorRotation` _sunlight (`KismetMathLibrary.MakeRotator` _returnvalue_2) false)
              (bind _moonlight (`local.MoonLight`)
                (:`then`
                  (`Actor.K2_SetActorRotation` _moonlight (`KismetMathLibrary.MakeRotator` (+ _returnvalue_2 180.0)) false))
                (:`else`))))
          (:`else`))))))
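; Blueprint function library for a day cycle that locates the sun and moon lights in the level.
; GetLights scans all DirectionalLight actors and returns those carrying the given sunlight and moonlight tags, checking the moon tag first.
; When several lights share a tag, the last match wins.
; NewFunction is an empty stub.
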(fn `GetLights`
  (params (SunlightTag :type "Name (by ref)") (MoonlightTag :type Name))
  (returns (SunLightRes :type "DirectionalLight Object Reference") (MoonLightRes :type "DirectionalLight Object Reference"))
  (locals (Moon :type "DirectionalLight Object Reference") (Sun :type "DirectionalLight Object Reference") (`SunlightTag Local` :type Name) (MoonlightTagLocal :type Name))
  (set `local.SunlightTag Local` SunlightTag)
  (set `local.MoonlightTagLocal` MoonlightTag)
  (bind _outactors (`GameplayStatics.GetAllActorsOfClass` null "/Script/Engine.DirectionalLight"))
  (for _array_element _outactors
    (if (`KismetArrayLibrary.Array_Contains` (`Actor.Tags` _array_element) (`local.MoonlightTagLocal`))
      (set `local.Moon` _array_element)
      (elif (`KismetArrayLibrary.Array_Contains` (`Actor.Tags` _array_element) (`local.SunlightTag Local`))
        (set `local.Sun` _array_element))))
  (return (`local.Sun`) (`local.Moon`)))

(fn `NewFunction`)
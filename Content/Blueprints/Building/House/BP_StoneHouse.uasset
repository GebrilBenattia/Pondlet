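; BP_StoneHouse is a stone house building that switches between basic, dark and light color palettes and highlights on hover.
; BeginPlay assigns the change-mesh material, then runs the basic palette, which creates a dynamic material instance and sets its BaseColor.
; The dark and light palette events only recolor that existing instance.
; Hover events call the parent and swap outline overlay materials, with a debug print on hover start.
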(event `self.SetBasicPalette`
  (set `self.Color` (struct :`R` 1.0 :`G` 0.987674 :`B` 0.126427 :`A` 1.0) :!label _label)
  (bind _returnvalue (`PrimitiveComponent.CreateDynamicMaterialInstance` (`self.StaticMeshComponent`) 0 "/Game/Assets/Materials/House/M_I_BP_ChangeMesh_01.M_I_BP_ChangeMesh_01" "None"))
  (`MaterialInstanceDynamic.SetVectorParameterValue` _returnvalue (`self.Base Color`) (`self.Color`)))

(event `self.ReceiveBeginPlay`
  (`PrimitiveComponent.SetMaterial` (`self.StaticMeshComponent`) 0 "/Game/Assets/Materials/House/M_I_BP_ChangeMesh_01.M_I_BP_ChangeMesh_01")
  (goto _label))

(event `self.SetDarkPalette`
  (set `self.Color` (struct :`R` 0.16141 :`G` 0.910288 :`B` 1.0 :`A` 1.0))
  (`MaterialInstanceDynamic.SetVectorParameterValue` (stale `self.SetBasicPalette` _returnvalue) (`self.Base Color`) (`self.Color`)))

(event `self.OnHoverEnd`
  (`parent.OnHoverEnd`)
  (`MeshComponent.SetOverlayMaterial` (`self.StaticMeshComponent`) "/Game/Assets/Materials/House/M_I_Outline_HouseNoHover.M_I_Outline_HouseNoHover"))

(event `self.SetLightPalette`
  (set `self.Color` (struct :`R` 1.0 :`G` 0.239298 :`B` 0.259195 :`A` 1.0))
  (`MaterialInstanceDynamic.SetVectorParameterValue` (stale `self.SetBasicPalette` _returnvalue) (`self.Base Color`) (`self.Color`)))

(event `self.OnHover`
  (`parent.OnHover`)
  (`MeshComponent.SetOverlayMaterial` (`self.StaticMeshComponent`) "/Game/Assets/Materials/House/M_I_Outline_HouseHover.M_I_Outline_HouseHover")
  (`KismetSystemLibrary.PrintString` "HOVER"))

(fn `UserConstructionScript`)
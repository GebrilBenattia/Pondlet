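; BP_StoneBoat is a building Blueprint that tints its StoneBoat mesh component when play begins.
; BeginPlay assigns the M_I_BP_ChangeMesh_01 material to slot 0, creates a dynamic instance from it and sets the BaseColor parameter to a dark purple.
; Two alternative tints, a red and a cyan, remain in the graph but never run, and the construction script is empty.
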(event `self.ReceiveBeginPlay`
  (bind _stoneboat (`self.StoneBoat`))
  (`PrimitiveComponent.SetMaterial` _stoneboat 0 "/Game/Assets/Materials/House/M_I_BP_ChangeMesh_01.M_I_BP_ChangeMesh_01")
  (set `self.Color` (struct :`R` 0.162029 :`G` 0.099899 :`B` 0.171441 :`A` 1.0))
  (bind _returnvalue (`PrimitiveComponent.CreateDynamicMaterialInstance` _stoneboat 0 "/Game/Assets/Materials/House/M_I_BP_ChangeMesh_01.M_I_BP_ChangeMesh_01" "None"))
  (`MaterialInstanceDynamic.SetVectorParameterValue` _returnvalue (`self.Base Color`) (`self.Color`)))

(fn `UserConstructionScript`)
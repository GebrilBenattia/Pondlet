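; BP_HiveSpawn is a building actor that spawns a hive matching the house preset.
; On BeginPlay it reads PresetFloat from the first BP_HouseSpawn in the level, truncates it and sets its ChildActor class to the wood or stone hive.
; The third preset also uses the stone hive, although disconnected debug prints label it Japanese.
; The HivePlaced event is empty.
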(event `HivePlaced`)

(event `self.ReceiveBeginPlay`
  (bind _childactor (`self.ChildActor`))
  (bind _outactors (`GameplayStatics.GetAllActorsOfClass` "/Game/Blueprints/Building/House/BP_HouseSpawn.BP_HouseSpawn_C"))
  (switch `int` (`KismetMathLibrary.FTrunc` (`/Game/Blueprints/Building/House/BP_HouseSpawn.PresetFloat` (`|GetArrayItem` _outactors)))
    (:`0`
      (`ChildActorComponent.SetChildActorClass` _childactor "/Game/Blueprints/Building/House/BP_WoodHive.BP_WoodHive_C"))
    (:`1`
      (`ChildActorComponent.SetChildActorClass` _childactor "/Game/Blueprints/Building/House/BP_StoneHive.BP_StoneHive_C"))
    (:`2`
      (`ChildActorComponent.SetChildActorClass` _childactor "/Game/Blueprints/Building/House/BP_StoneHive.BP_StoneHive_C"))))

(fn `UserConstructionScript`)
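; Birdhouse building that shows a style-matched house model and periodically spawns birds around itself.
; On BeginPlay and preset change, it reads PresetFloat from the first BP_HouseSpawn in the level and sets its child actor to the wood, stone or Japanese birdhouse.
; A looping timer runs SpawnAnimal, which extends the parent version by spawning a VFX and bird at a random nearby point and recording the bird in SpawnedActors.
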(event `self.OnPresetChange`
  (bind _childactor (`self.ChildActor`))
  (bind _outactors (`GameplayStatics.GetAllActorsOfClass` "/Game/Blueprints/Building/House/BP_HouseSpawn.BP_HouseSpawn_C" :!label _label))
  (switch `int` (`KismetMathLibrary.FTrunc` (`/Game/Blueprints/Building/House/BP_HouseSpawn.PresetFloat` (`|GetArrayItem` _outactors)))
    (:`0`
      (`ChildActorComponent.SetChildActorClass` _childactor "/Game/Blueprints/Building/House/BP_Wood_BirdHouse.BP_Wood_BirdHouse_C"))
    (:`1`
      (`ChildActorComponent.SetChildActorClass` _childactor "/Game/Blueprints/Building/House/BP_Stone_BirdHouse.BP_Stone_BirdHouse_C"))
    (:`2`
      (`ChildActorComponent.SetChildActorClass` _childactor "/Game/Blueprints/Building/House/BP_Japanese_BirdHouse.BP_Japanese_BirdHouse_C"))))

(event `self.ReceiveBeginPlay`
  (`parent.ReceiveBeginPlay`)
  (`KismetSystemLibrary.K2_SetTimer` null "SpawnAnimal" 5.0 true)
  (goto _label))

(fn `SpawnAnimal`
  (locals (NewLocalVar :type "Vector Structure"))
  (`parent.SpawnAnimal`)
  (bind _output_get (set `local.NewLocalVar` (+ (`self.K2_GetActorLocation`) (* (`KismetMathLibrary.RandomUnitVector`) (`KismetMathLibrary.RandomIntegerInRange` 0 300)))))
  (`|SpawnActorFromClass` "/Game/Blueprints/AI/Species/BP_SpawnVFX.BP_SpawnVFX_C" (`KismetMathLibrary.MakeTransform` _output_get (struct) (3.5 3.5 3.5)) "Undefined" "MultiplyWithRoot" null null)
  (bind _returnvalue (`|SpawnActorFromClass` "/Game/Blueprints/AI/Species/BP_BirdTMP.BP_BirdTMP_C" (`KismetMathLibrary.MakeTransform` _output_get (`self.RandRot`) (3.5 3.5 3.5)) "Undefined" "MultiplyWithRoot" null null))
  (`KismetArrayLibrary.Array_Add` (`self.SpawnedActors`) _returnvalue))

(fn `UserConstructionScript`)
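; BP_Addon is a house addon actor that appears to serve as a base, with empty OnPresetChange and SpawnAnimal hooks.
; On BeginPlay it finds the BP_HouseSpawn actor and binds OnPresetChange to its preset change event.
; Despawn plays a Niagara effect, destroys the tracked spawned actors, then itself.
; Helpers return a random yaw rotation and spawn a scaled-up BP_SpawnVFX at the addon's location.
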(event `self.ReceiveBeginPlay`
  (bind _returnvalue (`GameplayStatics.GetActorOfClass` "/Game/Blueprints/Building/House/BP_HouseSpawn.BP_HouseSpawn_C"))
  (add `/Game/Blueprints/Building/House/BP_HouseSpawn.PresetChange` _returnvalue (delegate `OnPresetChange`)))

(event `OnPresetChange`)

(fn `CallSpawnVFX`
  (bind _returnvalue_location (`KismetMathLibrary.BreakTransform` (`self.GetTransform`)))
  (`|SpawnActorFromClass` "/Game/Blueprints/AI/Species/BP_SpawnVFX.BP_SpawnVFX_C" (`KismetMathLibrary.MakeTransform` _returnvalue_location (struct) (3.5 3.5 3.5)) "Undefined" "MultiplyWithRoot" null null))

(fn `Despawn`
  (`NiagaraFunctionLibrary.SpawnSystemAtLocation` (`self.DespawnNiagara`) (`self.K2_GetActorLocation`))
  (for _array_element (`self.SpawnedActors`)
    (`self.K2_DestroyActor` _array_element))
  (`self.K2_DestroyActor`))

(fn `RandRot`
  (returns (ReturnValue :type "Rotator Structure"))
  (return (`KismetMathLibrary.MakeRotator` 0.0 0.0 (`KismetMathLibrary.Conv_IntToDouble` (`KismetMathLibrary.RandomInteger` 360)))))

(fn `SpawnAnimal`)

(fn `UserConstructionScript`)
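; BP_HouseTest is a test house Blueprint that switches between wood, stone and bamboo looks and three color palettes.
; It holds three house meshes (Wood, Provence, Japanese), and each Trigger event shows one and hides the other two.
; Dark, Medium and Light palette events set material slot 0 on all three meshes, so the palette carries across style changes.
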(event `Trigger_WoodHouse`
  ;[1 1 1] Mesh Visibility Switch
  (`SceneComponent.SetVisibility` (`self.SM_ProvenceHouse`) false false)
  (`SceneComponent.SetVisibility` (`self.SM_JapaneseHouse`) false false)
  (`SceneComponent.SetVisibility` (`self.SM_WoodHouse`) true false))

(event `Trigger_StoneHouse`
  ;[1 1 1] Mesh Visibility Switch
  (`SceneComponent.SetVisibility` (`self.SM_WoodHouse`) false false)
  (`SceneComponent.SetVisibility` (`self.SM_JapaneseHouse`) false false)
  (`SceneComponent.SetVisibility` (`self.SM_ProvenceHouse`) true false))

(event `Trigger_BambooHouse`
  ;[1 1 1] Mesh Visibility Switch
  (`SceneComponent.SetVisibility` (`self.SM_ProvenceHouse`) false false)
  (`SceneComponent.SetVisibility` (`self.SM_WoodHouse`) false false)
  (`SceneComponent.SetVisibility` (`self.SM_JapaneseHouse`) true false))

(event `DarkPaletteSwitch`
  ;[1 1 1] MaterialSwitch
  (`PrimitiveComponent.SetMaterial` (`self.SM_JapaneseHouse`) 0 "/Game/Assets/Materials/House/M_I_BP_ChangeMesh_01.M_I_BP_ChangeMesh_01")
  (`PrimitiveComponent.SetMaterial` (`self.SM_ProvenceHouse`) 0 "/Game/Assets/Materials/House/M_I_BP_ChangeMesh_01.M_I_BP_ChangeMesh_01")
  (`PrimitiveComponent.SetMaterial` (`self.SM_WoodHouse`) 0 "/Game/Assets/Materials/House/M_I_BP_ChangeMesh_01.M_I_BP_ChangeMesh_01"))

(event `MediumPaletteSwitch`
  ;[1 1 1] MaterialSwitch
  (`PrimitiveComponent.SetMaterial` (`self.SM_WoodHouse`) 0 "/Game/Assets/Materials/House/M_I_BP_ChangeMesh_02.M_I_BP_ChangeMesh_02")
  (`PrimitiveComponent.SetMaterial` (`self.SM_ProvenceHouse`) 0 "/Game/Assets/Materials/House/M_I_BP_ChangeMesh_02.M_I_BP_ChangeMesh_02")
  (`PrimitiveComponent.SetMaterial` (`self.SM_JapaneseHouse`) 0 "/Game/Assets/Materials/House/M_I_BP_ChangeMesh_02.M_I_BP_ChangeMesh_02"))

(event `LightPaletteSwitch`
  ;[1 1 1] MaterialSwitch
  (`PrimitiveComponent.SetMaterial` (`self.SM_WoodHouse`) 0 "/Game/Assets/Materials/House/M_I_BP_ChangeMesh_03.M_I_BP_ChangeMesh_03")
  (`PrimitiveComponent.SetMaterial` (`self.SM_ProvenceHouse`) 0 "/Game/Assets/Materials/House/M_I_BP_ChangeMesh_03.M_I_BP_ChangeMesh_03")
  (`PrimitiveComponent.SetMaterial` (`self.SM_JapaneseHouse`) 0 "/Game/Assets/Materials/House/M_I_BP_ChangeMesh_03.M_I_BP_ChangeMesh_03"))

(fn `UserConstructionScript`)
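; BP_WoodLantern is a wooden lantern building prop that tints its mesh when play begins.
; On BeginPlay it assigns the ChangeMesh material to the lantern, creates a dynamic material instance from it and sets the BaseColor parameter to yellow.
; Disconnected nodes hold alternative red and cyan tints that never run.
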(event `self.ReceiveBeginPlay`
  (bind _woodlantern (`self.WoodLantern`))
  (`PrimitiveComponent.SetMaterial` _woodlantern 0 "/Game/Assets/Materials/House/M_I_BP_ChangeMesh_01.M_I_BP_ChangeMesh_01")
  (set `self.Color` (struct :`R` 1.0 :`G` 0.987674 :`B` 0.126427 :`A` 1.0))
  (bind _returnvalue (`PrimitiveComponent.CreateDynamicMaterialInstance` _woodlantern 0 "/Game/Assets/Materials/House/M_I_BP_ChangeMesh_01.M_I_BP_ChangeMesh_01" "None"))
  (`MaterialInstanceDynamic.SetVectorParameterValue` _returnvalue (`self.Base Color`) (`self.Color`)))

(fn `UserConstructionScript`)
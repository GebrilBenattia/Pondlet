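; BP_BoatSpawn is a building spawner actor that shows a wood, stone or Japanese boat through its ChildActor component.
; On BeginPlay it reads PresetFloat from the first BP_HouseSpawn in the level and sets the child actor class to the matching boat.
; BoatWoodPreset, BoatStonePreset and BoatJapanesePreset events switch the boat class directly, reusing the same branches.
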(event `self.ReceiveBeginPlay`
  (bind _childactor (`self.ChildActor`))
  (bind _outactors (`GameplayStatics.GetAllActorsOfClass` "/Game/Blueprints/Building/House/BP_HouseSpawn.BP_HouseSpawn_C"))
  (switch `int` (`KismetMathLibrary.FTrunc` (`/Game/Blueprints/Building/House/BP_HouseSpawn.PresetFloat` (`|GetArrayItem` _outactors)))
    (:`0`
      (`ChildActorComponent.SetChildActorClass` _childactor "/Game/Blueprints/Building/House/BP_WoodBoat.BP_WoodBoat_C" :!label _label))
    (:`1`
      (`ChildActorComponent.SetChildActorClass` _childactor "/Game/Blueprints/Building/House/BP_StoneBoat.BP_StoneBoat_C" :!label _label_2))
    (:`2`
      (`ChildActorComponent.SetChildActorClass` _childactor "/Game/Blueprints/Building/House/BP_JapaneseBoat.BP_JapaneseBoat_C" :!label _label_3))))

(event `BoatWoodPreset`
  (goto _label))

(event `BoatStonePreset`
  (goto _label_2))

(event `BoatJapanesePreset`
  (goto _label_3))

(fn `UserConstructionScript`)
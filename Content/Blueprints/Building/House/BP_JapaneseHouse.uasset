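; BP_JapaneseHouse is a Japanese house building with switchable color palettes and a hover outline.
; BeginPlay applies the base material, then runs the basic palette, which creates a dynamic material instance and tints its BaseColor.
; Dark and light palette events recolor that same instance, while the basic event recreates it on each call.
; Hover events swap overlay outline materials, with hover-on also printing a debug string.
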(event `SetJHouseBasicPalette`
  (set `self.Color` (struct :`R` 1.0 :`G` 0.987674 :`B` 0.126427 :`A` 1.0) :!label _label)
  (bind _returnvalue (`PrimitiveComponent.CreateDynamicMaterialInstance` (`self.SM_JapaneseHouse`) 0 "/Game/Assets/Materials/House/M_I_BP_ChangeMesh_01.M_I_BP_ChangeMesh_01" "None"))
  (`MaterialInstanceDynamic.SetVectorParameterValue` _returnvalue (`self.Base Color`) (`self.Color`)))

(event `self.ReceiveBeginPlay`
  (`PrimitiveComponent.SetMaterial` (`self.SM_JapaneseHouse`) 0 "/Game/Assets/Materials/House/M_I_BP_ChangeMesh_01.M_I_BP_ChangeMesh_01")
  (goto _label))

(event `SetJHouseDarkPalette`
  (set `self.Color` (struct :`R` 0.16141 :`G` 0.910288 :`B` 1.0 :`A` 1.0))
  (`MaterialInstanceDynamic.SetVectorParameterValue` (stale `SetJHouseBasicPalette` _returnvalue) (`self.Base Color`) (`self.Color`)))

(event `JapaneseHouseHoverOff`
  (`MeshComponent.SetOverlayMaterial` (`self.SM_JapaneseHouse`) "/Game/Assets/Materials/House/M_I_Outline_HouseNoHover.M_I_Outline_HouseNoHover"))

(event `SetJHouseLightPalette`
  (set `self.Color` (struct :`R` 1.0 :`G` 0.239298 :`B` 0.259195 :`A` 1.0))
  (`MaterialInstanceDynamic.SetVectorParameterValue` (stale `SetJHouseBasicPalette` _returnvalue) (`self.Base Color`) (`self.Color`)))

(event `JapaneseHouseHoverOn`
  (`MeshComponent.SetOverlayMaterial` (`self.SM_JapaneseHouse`) "/Game/Assets/Materials/House/M_I_Outline_HouseHover.M_I_Outline_HouseHover")
  (`KismetSystemLibrary.PrintString` "HOVER"))

(fn `UserConstructionScript`)
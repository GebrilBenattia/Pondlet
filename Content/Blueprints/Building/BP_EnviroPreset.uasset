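; BP_EnviroPreset is a building-system actor that switches the ground material on its static mesh between environment presets.
; BeginPlay assigns the green ground material by slot name.
; Custom events for Stone, Wood and Bamboo presets set element 0 to yellow, green or pink ground materials and print a grass-color label.
; The Stone preset prints "Gray Grass" despite applying the yellow material.
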(event `self.ReceiveBeginPlay`
  (`PrimitiveComponent.SetMaterialByName` (`self.StaticMesh`) "None" "/Game/Assets/Materials/House/MI_Ground_Green.MI_Ground_Green"))

(event `Trigger_StonePreset`
  ;[1 1 1] Custom Color Change Events
  (`PrimitiveComponent.SetMaterial` (`self.StaticMesh`) 0 "/Game/Assets/Materials/House/MI_Yellow_Ground.MI_Yellow_Ground")
  (`KismetSystemLibrary.PrintString` "Gray Grass"))

(event `Trigger_WoodPreset`
  ;[1 1 1] Custom Color Change Events
  (`PrimitiveComponent.SetMaterial` (`self.StaticMesh`) 0 "/Game/Assets/Materials/House/MI_Ground_Green.MI_Ground_Green")
  (`KismetSystemLibrary.PrintString` "Green Grass"))

(event `Trigger_BambooPreset`
  ;[1 1 1] Custom Color Change Events
  (`PrimitiveComponent.SetMaterial` (`self.StaticMesh`) 0 "/Game/Assets/Materials/House/MI_Pink_Ground.MI_Pink_Ground")
  (`KismetSystemLibrary.PrintString` "Pink Grass"))

(fn `UserConstructionScript`)
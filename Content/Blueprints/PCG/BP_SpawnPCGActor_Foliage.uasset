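; Actor that caches PCG-generated foliage points and spawns items at random spots among them.
; When its PCG component finishes generating, it reads point data from the "MeshPoints" output pin and stores the locations in a Points array, clearing it for each matching data entry.
; SpawnGroundItem picks a random cached location, then spawns the given class plus a BP_SpawnVFXBuildngs effect actor there.
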(event OnPCGGraphGeneratedExternal(PCGComponent)
  (params (PCGComponent :type PCG%20Component%20Object%20Reference))
  (for _array_element (.taggeddata (Class|PCGComponent|GetGeneratedGraphOutput PCGComponent))
    (if (== (.pin _array_element) "MeshPoints")
      (bind _aspcgpoint_data (Utilities|Casting|CastToPCGPointData (.data _array_element)))
      (Utilities|Array|Clear (Variables|Default|GetPoints))
      (for _array_element_2 (SpatialData|GetPoints _aspcgpoint_data)
        (Utilities|Array|Add (Variables|Default|GetPoints) (.Location (Math|Transform|BreakTransform (.transform _array_element_2))))))))

(event EventBeginPlay
  (|CallParentFunction) ; This node is disabled and will not be called.\nDrag off pins to build functionality.
)

(event Collision|EventActorBeginOverlap
  (params (OtherActor :type Actor%20Object%20Reference)))

(event EventTick
  (params (DeltaSeconds :type Float%20%28single-precision%29))
  (|CallParentFunction DeltaSeconds) ; This node is disabled and will not be called.\nDrag off pins to build functionality.
)

(fn ConstructionScript
  (|CallParentFunction))

(fn SpawnGroundItem
  (params (Class :type BP%20Addon%20Class%20Reference))
  (bind _output_get (LocalVariables|SetNewLocalVar (Utilities|Array|Get(acopy) (Variables|Default|GetPoints) (Math|Random|RandomIntegerinRange 0 (- (Utilities|Array|Length (Variables|Default|GetPoints)) 1)))))
  (Game|SpawnActorfromClass Class (Math|Transform|MakeTransform _output_get "0, 0, 0" "1.000000,1.000000,1.000000") "Undefined" "MultiplyWithRoot" 0 0)
  (Game|SpawnActorfromClass "/Game/Blueprints/Building/House/BP_SpawnVFXBuildngs.BP_SpawnVFXBuildngs_C" (Math|Transform|MakeTransform _output_get "0, 0, 0" "1.000000,1.000000,1.000000") "Undefined" "OverrideRootScale" 0 0))
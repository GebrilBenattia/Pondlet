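; BP_Pond is a pond actor that publishes its position and extent to the LandscapeModifier material parameter collection.
; Every Tick, it writes its world location to PondCenter and its MaxDistance variable to PondMaxDistance, exposing both to any material that reads the collection.
; Both values are global to the collection, so multiple pond instances would overwrite each other.
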(event `self.ReceiveBeginPlay`)

(event `self.ReceiveTick`
  (params (DeltaSeconds :type "Float (single-precision)"))
  (`KismetMaterialLibrary.SetVectorParameterValue` (`self.LandscapeModifier`) "PondCenter" (`KismetMathLibrary.Conv_VectorToLinearColor` (`self.K2_GetActorLocation`)))
  (`KismetMaterialLibrary.SetScalarParameterValue` (`self.LandscapeModifier`) "PondMaxDistance" (`self.MaxDistance`)))

(fn `UserConstructionScript`
  (`parent.UserConstructionScript`))
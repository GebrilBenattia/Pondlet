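; Pond actor that shapes landscape by spawning patch actors from PCG point data.
; When PCGDigging finishes generating, it destroys all existing patches in the level, then reads the PondDigging and PondOutline pins.
; Digging points become patches lowered by their DistanceToSides attribute, capped and scaled, while outline points become tight patches offset by OutlineHeight.
; Alternate callbacks and deepest-point search helpers remain outside that main path.
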(event OnPCGGraphGeneratedExternal(PCGDigging)
  (params (PCGComponent :type PCG%20Component%20Object%20Reference))
  (Development|PrintString "Hello")
  (CallFunction|PCGMetadataKeyTest))

(event EventBeginPlay)

(event Collision|EventActorBeginOverlap
  (params (OtherActor :type Actor%20Object%20Reference)))

(event EventTick
  (params (DeltaSeconds :type Float%20%28single-precision%29)))

(fn ConstructionScript
  (|CallParentFunction))

(fn PCGMetadataKeyTest
  (params (NewParam :type PCG%20Data%20Collection%20Structure))
  (Utilities|FlowControl|Sequence
    (:then_0
      (bind _outactors (Actor|GetAllActorsOfClass "/Game/Blueprints/BP_LandscapePatch.BP_LandscapePatch_C"))
      (for _array_element _outactors
        (Actor|DestroyActor _array_element))
      (bind _outactors_2 (Actor|GetAllActorsOfClass "/Game/Blueprints/BP_LandscapePatchBorders.BP_LandscapePatchBorders_C"))
      (for _array_element_2 _outactors_2
        (Actor|DestroyActor _array_element_2))
      (bind _outactors_3 (Actor|GetAllActorsOfClass "/Game/Blueprints/BP_LandscapePatchActor.BP_LandscapePatchActor_C"))
      (for _array_element_3 _outactors_3
        (Actor|DestroyActor _array_element_3)))
    (:then_1
      (bind _returnvalue (Data|GetInputsbyPinLabel NewParam "PondDigging"))
      (bind _aspcgpoint_data (Utilities|Casting|CastToPCGPointData (.Data (Utilities|Struct|BreakPCGTaggedData (Utilities|Array|Get(acopy) _returnvalue)))))
      (LocalVariables|SetPCGPointData _aspcgpoint_data)
      (bind _returnvalue_2 (Data|GetInputsbyPinLabel NewParam "PondOutline"))
      (bind _aspcgpoint_data_2 (Utilities|Casting|CastToPCGPointData (.Data (Utilities|Struct|BreakPCGTaggedData (Utilities|Array|Get(acopy) _returnvalue_2)))))
      (LocalVariables|SetOutlinePointData _aspcgpoint_data_2))
    (:then_2
      (bind _pcgpointdata (LocalVariables|GetPCGPointData)
        (:then
          (for _array_element_4 (SpatialData|GetPoints _pcgpointdata)
            (bind _returnvalue_3 (CallFunction|PointtoDepth _array_element_4 (LocalVariables|GetPCGPointData)))
            (Game|SpawnActorfromClass "/Game/Blueprints/BP_LandscapePatchActor.BP_LandscapePatchActor_C" (Math|Transform|MakeTransform (+ _returnvalue_3 (.location (.Transform (Utilities|Struct|BreakPCGPoint _array_element_4)))) (.rotation (.Transform (Utilities|Struct|BreakPCGPoint _array_element_4))) (.scale (.Transform (Utilities|Struct|BreakPCGPoint _array_element_4)))) "Undefined" "MultiplyWithRoot" 0 1e+02 2e+02 0)))
        (:else)))
    (:then_3
      (bind _outlinepointdata (LocalVariables|GetOutlinePointData)
        (:then
          (CallFunction|OutlinePointGeneration _outlinepointdata))
        (:else)))))

(fn PointtoDepth
  (params (PCGPoint :type PCG%20Point%20Structure) (PCGPointData :type PCG%20Point%20Data%20Object%20Reference))
  (bind _returnvalue (Ability|Attribute|GetFloatAttribute PCGPoint (Metadata|ConstMetadata PCGPointData) "DistanceToSides"))
  (return (Math|Vector|MakeVector 0.0 0.0 (* (Math|Float|Min(Float) (Variables|Default|GetMaxDepth) _returnvalue) (Variables|Default|GetDistanceToDepthMultiplier) -1.0))))

(fn PCGFirstCallback
  (params (NewParam :type PCG%20Data%20Collection%20Structure))
  (bind _pcgdigging (Variables|Default|GetPCGDigging))
  (Class|PCGComponent|NotifyPropertiesChangedfromBlueprint _pcgdigging)
  (PCG|Generate _pcgdigging false))

(fn SpawnLandscapePatch
  (params (Points :type Array%20of%20PCG%20Point%20Structures) (Data :type PCG%20Point%20Data%20Object%20Reference))
  (for _array_element Points
    (bind _output_get (LocalVariables|SetCurrentPoint _array_element))
    (bind _depth (CallFunction|PointtoDepthFloat _output_get Data))
    (LocalVariables|SetCurrentDepth _depth)
    (if (or (== (LocalVariables|GetCurrentDepth) -1.0) (<= (LocalVariables|GetLocqlMaxDepth) (LocalVariables|GetCurrentDepth)))
      (LocalVariables|SetLocqlMaxDepth (LocalVariables|GetCurrentDepth))
      (LocalVariables|SetFarthestPoint (LocalVariables|GetCurrentPoint))))
  (Development|PrintString (Utilities|String|ToString(Float) (LocalVariables|GetLocqlMaxDepth)))
  (return (LocalVariables|GetFarthestPoint)))

(fn PointtoDepthFloat
  (params (PCGPoint :type PCG%20Point%20Structure) (PCGPointData :type PCG%20Point%20Data%20Object%20Reference))
  (bind _returnvalue (Ability|Attribute|GetFloatAttribute PCGPoint (Metadata|ConstMetadata PCGPointData) "DistanceToSides"))
  (return _returnvalue))

(fn PCGCallback2
  (params (NewParam :type PCG%20Data%20Collection%20Structure))
  (Utilities|FlowControl|Sequence
    (:then_0
      (bind _outactors (Actor|GetAllActorsOfClass "/Game/Blueprints/BP_LandscapePatch.BP_LandscapePatch_C"))
      (for _array_element _outactors
        (Actor|DestroyActor _array_element)))
    (:then_1
      (bind _returnvalue (Data|GetInputsbyPinLabel NewParam "PondDigging"))
      (bind _aspcgpoint_data (Utilities|Casting|CastToPCGPointData (.Data (Utilities|Struct|BreakPCGTaggedData (Utilities|Array|Get(acopy) _returnvalue)))))
      (LocalVariables|SetPCGPointData _aspcgpoint_data))
    (:then_2
      (bind _pcgpointdata (LocalVariables|GetPCGPointData)
        (:then
          (for _array_element_2 (SpatialData|GetPoints _pcgpointdata)
            (Game|SpawnActorfromClass "/Game/Blueprints/BP_LandscapePatch.BP_LandscapePatch_C" (Math|Transform|MakeTransform (- (.location (Utilities|Struct|BreakPCGPoint _array_element_2)) "0.000000,0.000000,100.000000") "0, 0, 0" "1.000000,1.000000,1.000000") "Undefined" "MultiplyWithRoot" 0 0)))
        (:else)))))

(fn SpawnLandscapePatch0
  (params (Points :type Array%20of%20PCG%20Point%20Structures) (Data :type PCG%20Point%20Data%20Object%20Reference))
  (for _array_element Points
    (bind _output_get (LocalVariables|SetCurrentPoint _array_element))
    (bind _depth (CallFunction|PointtoDepthFloat _output_get Data))
    (LocalVariables|SetCurrentDepth _depth)
    (if (or (== (LocalVariables|GetCurrentDepth) -1.0) (<= (LocalVariables|GetLocqlMaxDepth) (LocalVariables|GetCurrentDepth)))
      (LocalVariables|SetLocqlMaxDepth (LocalVariables|GetCurrentDepth))
      (LocalVariables|SetFarthestPoint (LocalVariables|GetCurrentPoint))))
  (Development|PrintString (Utilities|String|ToString(Float) (LocalVariables|GetLocqlMaxDepth)))
  (return (LocalVariables|GetFarthestPoint)))

(fn OutlinePointGeneration
  (params (NewParam :type PCG%20Point%20Data%20Object%20Reference))
  (for _array_element (SpatialData|GetPoints NewParam)
    (Game|SpawnActorfromClass "/Game/Blueprints/BP_LandscapePatchActor.BP_LandscapePatchActor_C" (Math|Transform|MakeTransform (+ (.Location (Math|Transform|BreakTransform (Utilities|Struct|BreakPCGPoint _array_element))) (Math|Vector|MakeVector 0.0 0.0 (Variables|Default|GetOutlineHeight))) (.Rotation (Math|Transform|BreakTransform (Utilities|Struct|BreakPCGPoint _array_element))) (.Scale (Math|Transform|BreakTransform (Utilities|Struct|BreakPCGPoint _array_element)))) "Undefined" "MultiplyWithRoot" 0 1e+01 1.0 0)))
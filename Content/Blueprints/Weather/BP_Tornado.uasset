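; BP_Tornado is a weather actor that travels in a straight line toward the house spawn.
; On BeginPlay it finds the BP_HouseSpawn actor and stores the normalized direction to it.
; Each Tick it offsets itself by Direction times Speed without sweep or delta-time scaling, so movement is frame-rate dependent, and reapplies a fixed enlarged world scale to its Niagara effect.
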(event `self.ReceiveBeginPlay`
  (bind _returnvalue (`GameplayStatics.GetActorOfClass` "/Game/Blueprints/Building/House/BP_HouseSpawn.BP_HouseSpawn_C"))
  (set `self.Direction` (`KismetMathLibrary.Normal` (- (`self.K2_GetActorLocation` _returnvalue) (`self.K2_GetActorLocation`)))))

(event `self.ReceiveTick`
  (params (DeltaSeconds :type "Float (single-precision)"))
  (`self.K2_AddActorWorldOffset` (* (`self.Direction`) (`self.Speed`)) false true)
  (`SceneComponent.SetWorldScale3D` (`self.Niagara`) (20.0 20.0 20.0)))

(fn `UserConstructionScript`)